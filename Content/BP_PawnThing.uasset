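; Player pawn for a two-player networked box-clicking reaction game with scores, ready state and restart.
; On BeginPlay the locally controlled pawn caches the first box and BPP_Server actor, enables the cursor and creates the UI.
; Clicking the selected box triggers it and reports to GM_Server through server events, which also handle readiness.
; Client events update scores and average reaction time, show the win/lose screen and clear it on restart.
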(event `initUI`
  ; initUI
  (bind _returnvalue (`|CreateWidget` "/Game/WBP_UI.WBP_UI_C"))
  (bind _output_get (set `self.UI` _returnvalue))
  (`UserWidget.AddToViewport` _output_get 0)
  (`KismetSystemLibrary.PrintString` "set To ViewPort"))

(event `resetState`
  (set `self.isPlaying` true)
  (set `self.myScore` 0))

(event `initCurrBox`
  ; initCurrBox
  (bind _outactors (`GameplayStatics.GetAllActorsOfClass` "/Game/BP_BoxThing.BP_BoxThing_C"))
  (set `self.currBox` (`|GetArrayItem` _outactors)))

(event `initServer`
  ; initServer
  (bind _outactors (`GameplayStatics.GetAllActorsOfClass` "/Game/BPP_Server.BPP_Server_C"))
  (set `self.server` (`|GetArrayItem` _outactors)))

(event `initPlayerController`
  (bind _returnvalue (`GameplayStatics.GetPlayerController` 0))
  ; initPlayerController
  (set `PlayerController.bShowMouseCursor` true _returnvalue)
  (set `PlayerController.bEnableMouseOverEvents` true _returnvalue))

(event `plusScore`)

(event `pawnComm`
  (`KismetSystemLibrary.PrintString` "pawnComm"))

(event `plusScoreServer`
  (`/Engine/EditorBlueprintResources/StandardMacros.IncrementInt` (`self.myScore`)
    (:`  `
      (`/Game/BPP_Server.updateScores` (`self.server`)))))

(event `self.ReceiveBeginPlay`
  (if (== self (`Controller.K2_GetPawn` (`GameplayStatics.GetPlayerController` 0)))
    (`self.initServer`)
    (`self.initPlayerController`)
    (`self.initCurrBox`)
    (`self.initUI`)))

(event `Key|LeftMouseButton`
  (params (Key :type "Key Structure"))
  (bind _currbox (`self.currBox`))
  (:`Pressed`
    (if (and (`/Game/BP_BoxThing.isCursorOver` _currbox) (`/Game/BP_BoxThing.isSelected` _currbox))
      (`self.changeCubeServer` (`self.currBox`))
      (`/Engine/EditorBlueprintResources/StandardMacros.IncrementInt` (`self.myScore`)
        (:`  `
          (`self.SERVER_printScores` (`self.id`)))))))

(event `CLIENT_setId`
  (params (id :type Integer))
  (set `self.id` id))

(event `selectCubeServer`
  (params (SelectedBox :type "/Game/BP_BoxThing Object Reference"))
  (`/Engine/EditorBlueprintResources/StandardMacros.IsValid` SelectedBox
    (:`Is Valid`
      (`/Game/BP_BoxThing.selectThis` SelectedBox))))

(event `restartButtonLocal`
  (`self.resetState`)
  (`self.isButtonPressedRPC`))

(event `changeCubeServer`
  (params (SelectedBox :type "/Game/BP_BoxThing Object Reference"))
  (`/Engine/EditorBlueprintResources/StandardMacros.IsValid` SelectedBox
    (:`Is Valid`
      (`self.changeCube` SelectedBox))))

(event `SERVER_printScores`
  (params (id :type Integer))
  (set `self.id` id)
  (bind _asgm_server (cast `/Game/GM_Server` (`GameplayStatics.GetGameMode`)))
  (`/Game/GM_Server.updateScore` _asgm_server (`self.id`)))

(event `Key|Seven`
  (params (Key :type "Key Structure"))
  (:`Pressed`
    (`self.GM_ServerConnectionTest`)))

(event `isButtonPressedRPC`
  (`/Game/BPP_Server.resetStateServer` (`self.server`)))

(event `changeCube`
  (params (SelectedBox :type "/Game/BP_BoxThing Object Reference"))
  (`/Game/BP_BoxThing.clickThis` SelectedBox))

(event `GM_ServerConnectionTest`
  (bind _asgm_server (cast `/Game/GM_Server` (`GameplayStatics.GetGameMode`)))
  (`/Game/GM_Server.commTest` _asgm_server))

(event `changeUIScore`
  (`/Game/WBP_UI.updateText` (`self.UI`)))

(event `CLIENT_updateUIScore`
  (params (score1 :type "Array of Integer") (reactionTime :type Integer) (end :type Integer))
  (bind _ui (`self.UI`))
  (bind _endui (`self.endUI`))
  (`KismetSystemLibrary.PrintString` (`KismetStringLibrary.Conv_IntToString` end))
  (set `self.reactionTime` (+ (`self.reactionTime`) reactionTime))
  (`/Game/WBP_UI.setScores` _ui (`|GetArrayItem` score1) (`|GetArrayItem` score1 1))
  (`/Game/WBP_UI.updateReactionTime` _ui (/ (`self.reactionTime`) (`self.myScore`)))
  (if (not (== end 0))
    (bind _returnvalue (`|CreateWidget` "/Game/WBP_EndScreen.WBP_EndScreen_C"))
    (bind _output_get (set `self.endUI` _returnvalue))
    (`UserWidget.AddToViewport` _output_get 0)
    (if (== end 2)
      (`/Game/WBP_EndScreen.setYouWin` _endui)
      (else
        (`/Game/WBP_EndScreen.setYouLose` _endui)))
    (`self.setReady` false)))

(event `serverCall`
  (`/Game/BPP_Server.serverPrint` (`self.server`)))

(event `CLIENT_restart`
  (bind _endui (`self.endUI`))
  (bind _ui (`self.UI`))
  (set `self.reactionTime` 0)
  (set `self.myScore` 0)
  (`/Engine/EditorBlueprintResources/StandardMacros.IsValid` _endui
    (:`Is Valid`
      (`Widget.RemoveFromParent` _endui)
      (`/Game/WBP_UI.setScores` _ui 0 0)
      (`/Game/WBP_UI.setWaiting` _ui false))))

(event `setReady`
  (params (isReady :type Boolean))
  (bind _output_get (set `self.isReady` isReady))
  (`self.SERVER_setReady` _output_get))

(event `9call`
  (`self.serverCall`)
  (`KismetSystemLibrary.PrintString` "Who callin"))

(event `Key|Nine`
  (params (Key :type "Key Structure"))
  (:`Pressed`
    (`self.9call`)
    (`KismetSystemLibrary.PrintString` "Who callin")))

(event `SERVER_setReady`
  (params (isReady :type Boolean))
  (set `self.isReady` isReady)
  (bind _asgm_server (cast `/Game/GM_Server` (`GameplayStatics.GetGameMode`)))
  (`/Game/GM_Server.checkAllReady` _asgm_server))

(fn `getRandomBoxThing`
  (returns (Output :type "Actor Object Reference"))
  (bind _outactors (`GameplayStatics.GetAllActorsOfClass` "/Game/BP_BoxThing.BP_BoxThing_C"))
  (return (`|GetArrayItem` _outactors (`KismetMathLibrary.RandomIntegerInRange` 0 (- (`KismetArrayLibrary.Array_Length` _outactors) 1)))))

(fn `UserConstructionScript`)