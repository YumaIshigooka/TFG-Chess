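; Server game mode for a multiplayer reaction game that highlights random boxes and scores players up to a maximum.
; BeginPlay waits for the expected pawn count, assigns IDs, then loops at random intervals selecting a box, returning to waiting if the count changes.
; A ready check starts play.
; Score updates send clients the scores, the Tick-timed reaction time for the scorer and end state, then allow the next selection.
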(event `commTest`
  (`KismetSystemLibrary.PrintString` "commTest"))

(event `initPlayers`)

(event `self.ReceiveBeginPlay`
  (bind _outactors (`GameplayStatics.GetAllActorsOfClass` "/Game/BP_BoxThing.BP_BoxThing_C"))
  (set `self.boxes` _outactors)
  (`KismetSystemLibrary.Delay` 0.5 :!label _label)
  (bind _outactors_2 (`GameplayStatics.GetAllActorsOfClass` "/Game/BP_PawnThing.BP_PawnThing_C"))
  (if (== (`KismetArrayLibrary.Array_Length` _outactors_2) (`self.expectedPlayers`))
    (bind _output_get (set `self.players` _outactors_2))
    (`KismetSystemLibrary.Delay` 2.0)
    (for (_array_element _array_index) _output_get
      (`/Game/BP_PawnThing.CLIENT_setId` _array_element _array_index)
      (`/Game/BP_PawnThing.CLIENT_restart` _array_element))
    (`self.resetScores`)
    (if (and (`self.isPlaying`) (not (`self.isSelect`))) :!label _label_2
      (`self.changeColor`))
    (`KismetSystemLibrary.Delay` (`KismetMathLibrary.RandomFloatInRange` 1.0 1.5))
    (bind _outactors_3 (`GameplayStatics.GetAllActorsOfClass` "/Game/BP_PawnThing.BP_PawnThing_C"))
    (if (== (`KismetArrayLibrary.Array_Length` _outactors_3) (`self.expectedPlayers`))
      (goto _label_2)
      (else
        (goto _label)))
    (else
      (goto _label))))

(event `self.ReceiveTick`
  (params (DeltaSeconds :type "Float (single-precision)"))
  (if (`self.isPlaying`)
    (set `self.changeTime` (+ DeltaSeconds (`self.changeTime`)))))

(event `initTimer`)

(event `checkAllReady`
  (set `self.areReady` true)
  (for _array_element (`self.players`)
    (set `self.areReady` (and (`self.areReady`) (`/Game/BP_PawnThing.isReady` _array_element))))
  (if (`self.areReady`)
    (for (_array_element_2 _array_index) (`self.players`)
      (`KismetArrayLibrary.Array_Set` (`self.scores`) _array_index)
      (`/Game/BP_PawnThing.CLIENT_restart` _array_element_2)
      (set `self.isPlaying` true))))

(event `changeColor`
  (set `self.currBox` (`KismetMathLibrary.RandomInteger` (- (`KismetArrayLibrary.Array_Length` (`self.boxes`)) 1)))
  (for _array_element (`self.players`)
    (`/Game/BP_PawnThing.selectCubeServer` _array_element (`|GetArrayItem` (`self.boxes`) (`self.currBox`)))
    (set `self.isSelect` true)
    (set `self.changeTime` 0.0)))

(event `updateScore`
  (params (id :type Integer))
  (bind _scores (`self.scores`))
  (bind _result (`/Engine/EditorBlueprintResources/StandardMacros.IncrementInt` (`|GetArrayItem` _scores id))
    (:`  `
      (`KismetArrayLibrary.Array_Set` _scores id _result)
      (set `self.isPlaying` (not (== _result (`self.maxScore`))))
      (`self.updateUI` id))))

(event `resetScores`
  (bind _scores (`self.scores`))
  (for (_ _array_index) _scores
    (`KismetArrayLibrary.Array_Set` _scores _array_index)))

(event `updateUI`
  (params (id :type Integer))
  (bind _scores (`self.scores`))
  (bind _returnvalue (`KismetMathLibrary.Conv_BoolToInt` (not (`self.isPlaying`))))
  (for (_array_element _array_index) (`self.players`)
    (if (== id _array_index)
      (`/Game/BP_PawnThing.CLIENT_updateUIScore` _array_element _scores (`KismetMathLibrary.FTrunc` (* (`self.changeTime`) 1000.0)) (* _returnvalue 2))
      (else
        (`/Game/BP_PawnThing.CLIENT_updateUIScore` _array_element _scores 0 _returnvalue))))
  (set `self.isSelect` false))

(event `changeColor_OLD`
  (bind _server (`self.server`))
  (if (not (`/Game/BPP_Server.isSelect` _server))
    (`/Game/BPP_Server.changeCube_Server` _server)
    (set `/Game/BPP_Server.isSelect` true _server)))

(event `initServer`
  (bind _outactors (`GameplayStatics.GetAllActorsOfClass` "/Game/BPP_Server.BPP_Server_C"))
  (bind _output_get (set `self.server` (`|GetArrayItem` _outactors)))
  (set `/Game/BPP_Server.allPlayers` (`self.players`) _output_get))

(fn `UserConstructionScript`)