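; Player controller for the multiplayer chess game, handling mouse piece selection, match UI and background music.
; Left clicks select or deselect hovered pieces or send moves to hovered slots through the BP_ChessPlayer pawn's server RPC, while Tick drops disabled selections.
; BeginPlay starts music and indexes board slots by row and column.
; Events relay player ID and started state, show waiting, starting and player-left widgets, and play a slow-motion end screen.
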(event `setEndScreen`
  (params (isWin :type Boolean))
  (bind _bgm (`self.BGM`))
  (`/Engine/EditorBlueprintResources/StandardMacros.IsValid` _bgm
    (:`Is Valid`
      (`ActorComponent.SetActive` _bgm false false))
    (:`Is Not Valid`
      _))
  (`GameplayStatics.SetGlobalTimeDilation` 0.2)
  (`KismetSystemLibrary.Delay` 0.8)
  (`GameplayStatics.SetGlobalTimeDilation` 1.0)
  (bind _returnvalue (`|CreateWidget` "/Game/Chess/WBP_Chess_EndScreen.WBP_Chess_EndScreen_C"))
  (`/Game/Chess/WBP_Chess_EndScreen.setWon` _returnvalue isWin)
  (`UserWidget.AddToViewport` _returnvalue 0))

(event `joinGame`
  (params (player :type "/Game/Chess/PC_Chess Object Reference (by ref)"))
  (bind _asgm_chess (cast `/Game/Chess/GM_Chess` (`GameplayStatics.GetGameMode`)))
  (`/Game/Chess/GM_Chess.joinGame` _asgm_chess player))

(event `setWaitingUI`
  (params (set :type Boolean))
  (bind _waitingui (`self.waitingUI`))
  (if set
    (`/Engine/EditorBlueprintResources/StandardMacros.IsValid` (`self.waitingUI`)
      (:`Is Not Valid`
        (bind _returnvalue (`|CreateWidget` "/Game/UI_WaitingForPlayers.UI_WaitingForPlayers_C"))
        (bind _output_get (set `self.waitingUI` _returnvalue))
        (`UserWidget.AddToViewport` _output_get 0)))
    (else
      (`/Engine/EditorBlueprintResources/StandardMacros.IsValid` _waitingui
        (:`Is Valid`
          (`Widget.RemoveFromParent` _waitingui)
          (set `self.waitingUI` null))))))

(event `setID`
  (params (id :type Boolean))
  (set `self.id` id))

(event `cameraBack`)

(event `reloadLevel`
  (bind _playerpawn (`self.playerPawn`))
  (`/Engine/EditorBlueprintResources/StandardMacros.IsValid` _playerpawn
    (:`Is Valid`
      (`/Game/Chess/BP_ChessPlayer.SERVER_Restart` _playerpawn))
    (:`Is Not Valid`
      (`KismetSystemLibrary.PrintString` "Hello"))))

(event `MULTI_setID`
  (params (id :type Boolean))
  (bind _output_get (set `self.id` id))
  (`self.LOCAL_setID` _output_get))

(event `CLIENT_setID`
  (params (id :type Boolean))
  (set `self.id` id))

(event `LOCAL_setID`
  (params (NewParam :type Boolean))
  (set `self.id` NewParam))

(event `SERVER_setID`
  (params (id :type Boolean))
  (`self.MULTI_setID` id))

(event `setReady`
  (set `self.started` true))

(event `SERVER_setStarted`
  (params (started :type Boolean))
  (`self.MULTI_setStarted` started))

(event `restartMusic`
  (bind _bgm (`self.BGM`))
  (`/Engine/EditorBlueprintResources/StandardMacros.IsValid` _bgm
    (:`Is Valid`
      (`ActorComponent.SetActive` _bgm true true)
      (`KismetSystemLibrary.PrintString` "BGM Starting"))
    (:`Is Not Valid`
      (`KismetSystemLibrary.PrintString` "BGM Not Valid"))))

(event `MULTI_setStarted`
  (params (started :type Boolean))
  (set `self.started` started))

(event `removeWidget`
  (set `self.waitingUI` null)
  (set `self.started` true)
  (set `self.currPiece` null)
  (set `self.currPîeceHover` null)
  (set `self.currSlotHover` null))

(event `self.ReceiveBeginPlay`
  (bind _returnvalue (`GameplayStatics.SpawnSound2D` "/Game/SFX/Ingame_BGM.Ingame_BGM" 1.0 1.0 0.0 null))
  (set `self.BGM` _returnvalue)
  (set `self.bShowMouseCursor` true)
  (set `self.bEnableMouseOverEvents` true)
  (bind _asbp_chess_player (cast `/Game/Chess/BP_ChessPlayer` (`GameplayStatics.GetPlayerPawn` 0)))
  (set `self.playerPawn` _asbp_chess_player)
  (`self.getAllSlots`))

(event `setViewTarget`)

(event `getAllSlots`
  (bind _outactors (`GameplayStatics.GetAllActorsOfClass` "/Game/Chess/BP_ChessSlot.BP_ChessSlot_C"))
  (for _array_element _outactors
    (`KismetArrayLibrary.Array_Set` (`self.slots`) (`self.getCoordsIndex` (`/Game/Chess/BP_ChessSlot.row` _array_element) (`/Game/Chess/BP_ChessSlot.col` _array_element)) _array_element true)))

(event `self.ReceiveTick`
  (params (DeltaSeconds :type "Float (single-precision)"))
  (bind _currpiece (`self.currPiece`))
  (`/Engine/EditorBlueprintResources/StandardMacros.IsValid` _currpiece
    (:`Is Valid`
      (if (not (`/Game/Chess/BP_Pawn.enabled` _currpiece))
        (message `/Game/Chess/BPI_Pawn.select` (`self.currPiece`))
        (set `self.currPiece` null)))))

(event `Key|LeftMouseButton`
  (params (Key :type "Key Structure"))
  (bind _currpiece (`self.currPiece`))
  (bind `_currpîecehover` (`self.currPîeceHover`))
  (bind _currpiece_2 (`self.currPiece`))
  (:`Pressed`
    (`/Engine/EditorBlueprintResources/StandardMacros.IsValid` `_currpîecehover`
      (:`Is Valid`
        (message `/Game/Chess/BPI_Pawn.select` `_currpîecehover`)
        (`/Engine/EditorBlueprintResources/StandardMacros.IsValid` _currpiece
          (:`Is Valid`
            (if (== (`self.currPîeceHover`) _currpiece)
              (set `self.currPiece` null)
              (else
                (set `self.currPiece` (`self.currPîeceHover`) :!label _label))))
          (:`Is Not Valid`
            (goto _label))))
      (:`Is Not Valid`
        (`/Engine/EditorBlueprintResources/StandardMacros.IsValid` (`self.currSlotHover`)
          (:`Is Valid`
            (`/Engine/EditorBlueprintResources/StandardMacros.IsValid` _currpiece_2
              (:`Is Valid`
                (`/Game/Chess/BPI_Pawn.highlightValidSlots` _currpiece_2 false)
                (`/Game/Chess/BP_ChessPlayer.SERVER_move` (`self.playerPawn`) _currpiece_2 (`self.currSlotHover`))
                (`/Game/Chess/BPI_Pawn.select` (`self.currPiece`))
                (set `self.currPiece` null)))))))))

(event `closingLobby`
  (bind _returnvalue (`|CreateWidget` "/Game/Chess/PlayerLeft.PlayerLeft_C"))
  (`UserWidget.AddToViewport` _returnvalue 0))

(event `UI_GameStarting`
  (bind _returnvalue (`|CreateWidget` "/Game/Chess/GameStarting.GameStarting_C"))
  (`UserWidget.AddToViewport` _returnvalue 0))

(fn `UserConstructionScript`)