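; Game mode for two-player networked chess that runs the match from lobby to end screen and rematch.
; On BeginPlay it indexes board slots, waits for two controllers, assigns IDs and spawn transforms, then initializes each piece's valid moves.
; A polling delay loop refreshes validity during play; after EndGame it resets the board once both players restart.
; If the player count changes, it closes the lobby and opens the demo map.
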(event `joinGame`
  (params (player :type "/Game/Chess/PC_Chess Object Reference (by ref)"))
  (bind _returnvalue (`KismetArrayLibrary.Array_Add` (`self.playerControllers`) player))
  (bind _returnvalue_2 (`KismetMathLibrary.Conv_IntToBool` _returnvalue))
  (`/Game/Chess/PC_Chess.CLIENT_setID` player _returnvalue_2)
  (if (not _returnvalue_2)
    (`KismetSystemLibrary.PrintString` "setting UI")
    (`/Game/Chess/PC_Chess.setWaitingUI` player true))
  (`KismetSystemLibrary.PrintString` "Player Joined"))

(event `checkIDs`)

(event `initSlots`
  (bind _outactors (`GameplayStatics.GetAllActorsOfClass` "/Game/Chess/BP_ChessSlot.BP_ChessSlot_C"))
  (for _array_element _outactors
    (`KismetArrayLibrary.Array_Set` (`self.slots`) (`self.getCoordsIndex` (`/Game/Chess/BP_ChessSlot.row` _array_element) (`/Game/Chess/BP_ChessSlot.col` _array_element)) _array_element true)))

(event `leaveGame`
  (params (player :type "/Game/Chess/PC_Chess Object Reference (by ref)"))
  (`KismetArrayLibrary.Array_RemoveItem` (`self.playerControllers`) player))

(event `reloadLevel`
  (for _array_element (`self.playerControllers`)
    (`/Game/Chess/PC_Chess.reloadLevel` _array_element)
    (bind _outactors (`GameplayStatics.GetAllActorsOfClass` "/Game/Chess/BP_ChessSlot.BP_ChessSlot_C"))
    (for _array_element_2 _outactors
      (`/Game/Chess/BP_ChessSlot.setDefaults` _array_element_2))
    (bind _outactors_2 (`GameplayStatics.GetAllActorsOfClass` "/Game/Chess/BP_Pawn.BP_Pawn_C"))
    (for _array_element_3 _outactors_2
      (`/Game/Chess/BP_Pawn.setDefaults` _array_element_3))))

(event `reboot`
  (bind _playercontrollers (`self.playerControllers`))
  (`self.initSlots` :!label _label)
  (bind _outactors (`GameplayStatics.GetAllActorsOfClass` "/Game/Chess/PC_Chess.PC_Chess_C" :!label _label_2))
  (if (== (`KismetArrayLibrary.Array_Length` _outactors) 2)
    (for _array_element _outactors
      (`/Game/Chess/PC_Chess.setWaitingUI` _array_element true))
    (`KismetSystemLibrary.Delay` 1.0)
    (bind _outactors_2 (`GameplayStatics.GetAllActorsOfClass` "/Game/Chess/PC_Chess.PC_Chess_C"))
    (set `self.playerControllers` _outactors_2)
    (bind _outactors_3 (`GameplayStatics.GetAllActorsOfClass` "/Game/Chess/BP_ChessPlayer.BP_ChessPlayer_C"))
    (set `self.playerPawns` _outactors_3)
    (for (_array_element_2 _array_index) _playercontrollers
      (bind _returnvalue (`KismetMathLibrary.Conv_IntToBool` _array_index))
      (`/Game/Chess/PC_Chess.SERVER_setID` _array_element_2 _returnvalue)
      (`/Game/Chess/PC_Chess.setWaitingUI` _array_element_2 false)
      (`/Game/Chess/PC_Chess.UI_GameStarting` _array_element_2)
      (bind _asbp_chess_player (cast `/Game/Chess/BP_ChessPlayer` (`Controller.K2_GetPawn` _array_element_2)))
      (`/Game/Chess/BP_ChessPlayer.setTransformAt` _asbp_chess_player (`self.getPlayerStart` _returnvalue))
      (`KismetSystemLibrary.PrintString` "Set Transform At"))
    (`KismetSystemLibrary.Delay` 3.0)
    (for _array_element_3 _playercontrollers
      (`/Game/Chess/PC_Chess.SERVER_setStarted` _array_element_3 true))
    (`self.loadValidSlotsServer`)
    (set `self.started` true)
    (bind _outactors_4 (`GameplayStatics.GetAllActorsOfClass` "/Game/Chess/PC_Chess.PC_Chess_C" :!label _label_3))
    (if (== (`KismetArrayLibrary.Array_Length` _outactors_4) 2)
      (if (`self.started`)
        (`KismetSystemLibrary.Delay` 0.25)
        (`self.checkPawns`)
        (goto _label_3)
        (else
          (set `self.started` true :!label _label_4)
          (for _array_element_4 (`self.playerControllers`)
            (set `self.started` (and (`/Game/Chess/PC_Chess.started` _array_element_4) (`self.started`))))
          (if (`self.started`)
            (for _array_element_5 (`self.playerControllers`)
              (`/Game/Chess/PC_Chess.UI_GameStarting` _array_element_5))
            (`KismetSystemLibrary.Delay` 3.0)
            (`self.reloadLevel`)
            (goto _label_3)
            (else
              (`KismetSystemLibrary.Delay` 1.0)
              (bind _outactors_5 (`GameplayStatics.GetAllActorsOfClass` "/Game/Chess/PC_Chess.PC_Chess_C"))
              (if (== (`KismetArrayLibrary.Array_Length` _outactors_5) 2)
                (goto _label_4)
                (else
                  (`self.closingLobby`)))))))
      (else
        (`self.closingLobby`)))
    (else
      (for _array_element_6 _outactors
        (`/Game/Chess/PC_Chess.setWaitingUI` _array_element_6 true))
      (`KismetSystemLibrary.Delay` 0.25)
      (goto _label_2))))

(event `self.ReceiveBeginPlay`
  (set `self.bUseSeamlessTravel` true)
  (goto _label))

(event `loadValidSlotsServer`
  (bind _outactors (`GameplayStatics.GetAllActorsOfClass` "/Game/Chess/BP_Pawn.BP_Pawn_C"))
  (for _array_element _outactors
    (`/Game/Chess/BP_Pawn.initSlots` _array_element)
    (message `/Game/Chess/BPI_Pawn.updateValidSlots` _array_element)))

(event `checkPawns`
  (`/Game/Chess/BP_ChessPlayer.updateValidity` (`|GetArrayItem` (`self.playerPawns`))))

(event `endGame`
  (params (winner :type Boolean))
  (set `self.started` false)
  (for _array_element (`self.playerControllers`)
    (`/Game/Chess/PC_Chess.SERVER_setStarted` _array_element false)
    (`/Game/Chess/PC_Chess.setEndScreen` _array_element (!= (`/Game/Chess/PC_Chess.id` _array_element) winner))))

(event `closingLobby`
  (bind _outactors (`GameplayStatics.GetAllActorsOfClass` "/Game/Chess/PC_Chess.PC_Chess_C"))
  (for _array_element _outactors
    (`/Game/Chess/PC_Chess.closingLobby` _array_element))
  (`KismetSystemLibrary.Delay` 3.0)
  (`GameplayStatics.OpenLevelBySoftObjectPtr` "/Game/Chess/MAP_Demo.MAP_Demo"))

(event `SERVER_move`
  (params (pawnID :type Integer) (newSlotID :type Integer))
  (bind (_value _returnvalue) (`BlueprintMapLibrary.Map_Find` (`self.pieces`) pawnID))
  (bind _output (`|GetArrayItem` (`self.slots`) newSlotID))
  ;[0.15 0 0 0.5] Never Used
  (if _returnvalue
    (message `/Game/Chess/BPI_Pawn.updateValidSlots` _value)
    (if (`BlueprintSetLibrary.Set_Contains` (`/Game/Chess/BP_Pawn.validSlots` _value) _output)
      (message `/Game/Chess/BPI_Pawn.move` _value _output false))))

(fn `getPlayerStart`
  (params (playerID :type Boolean))
  (returns (transform :type "Transform Structure (by ref)"))
  (if playerID
    (bind _returnvalue (`GameplayStatics.GetActorOfClass` "/Game/Chess/spawnPoint2.spawnPoint2_C"))
    (return (`self.GetTransform` _returnvalue))
    (else
      (bind _returnvalue_2 (`GameplayStatics.GetActorOfClass` "/Game/Chess/spawnPoint.spawnPoint_C"))
      (return (`self.GetTransform` _returnvalue_2)))))

(fn `UserConstructionScript`)