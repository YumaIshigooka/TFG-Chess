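; Networked chess player Blueprint that relays moves, board state and restarts through SERVER and ALL events.
; A server move ends the game when the target holds a type 5 piece, and broadcasts moves to valid slots.
; updateValidity re-sends slot and piece values, throttled to every fourth pass unless recently changed.
; Restart resets all slots and pieces, clears widgets, flags the local controller as started and starts the in-game music.
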(event `setTransformAt`
  (params (NewTransform :type "Transform Structure (by ref)"))
  (bind _defaultsceneroot (`self.DefaultSceneRoot`))
  (`/Engine/EditorBlueprintResources/StandardMacros.IsValid` _defaultsceneroot
    (:`Is Valid`
      (`SceneComponent.K2_SetWorldTransform` _defaultsceneroot NewTransform false false))
    (:`Is Not Valid`
      (`KismetSystemLibrary.PrintString` "Nope"))))

(event `SERVER_move`
  (params (piece :type "/Game/Chess/BP_Pawn Object Reference") (slot :type "/Game/Chess/BP_ChessSlot Object Reference"))
  (bind _piecepawn (`/Game/Chess/BP_ChessSlot.piecePawn` slot))
  (if (`/Game/Chess/GM_Chess.started` (`self.As GM Chess`))
    (`/Engine/EditorBlueprintResources/StandardMacros.IsValid` _piecepawn
      (:`Is Valid`
        (if (!= (`/Game/Chess/BP_Pawn.type` _piecepawn) 5)
          (if (not (`/Game/Chess/GM_Chess.started` (`self.As GM Chess`))) :!label _label
            (`/Game/Chess/GM_Chess.endGame` (`self.As GM Chess`) (`/Game/Chess/BP_ChessSlot.isWhite` slot) :!label _label_2))
          (else
            (goto _label_2))))
      (:`Is Not Valid`
        (goto _label)))
    (if (`BlueprintSetLibrary.Set_Contains` (`/Game/Chess/BP_Pawn.validSlots` piece) slot)
      (message `/Game/Chess/BPI_Pawn.move` piece slot false)
      (`self.ALL_move` piece slot))))

(event `updateValidity`
  (`self.updateSlots`)
  (`self.updatePlayers` true))

(event `ALL_move`
  (params (piece :type "/Game/Chess/BP_Pawn Object Reference") (slot :type "/Game/Chess/BP_ChessSlot Object Reference"))
  (message `/Game/Chess/BPI_Pawn.move` piece slot true))

(event `self.ReceiveBeginPlay`
  (bind _asgm_chess (cast `/Game/Chess/GM_Chess` (`GameplayStatics.GetGameMode`)))
  (set `self.As GM Chess` _asgm_chess)
  (bind _aspc_chess (cast `/Game/Chess/PC_Chess` (`GameplayStatics.GetPlayerController` 0))
    (:`then`
      (set `self.As PC Chess` _aspc_chess))
    (:`CastFailed`
      (`KismetSystemLibrary.PrintString` "NO PC"))))

(event `SERVER_Restart`
  (`self.ALL_Restart`))

(event `setValuesThing`
  (params (bp_pawn :type "/Game/Chess/BP_Pawn Object Reference") (slot :type "/Game/Chess/BP_ChessSlot Object Reference") (moved :type Boolean) (enabled :type Boolean) (NewLocation :type "Vector Structure") (GeometryCollection :type "GeometryCollectionComponent Object Reference") (playerMove :type Boolean) (type :type Integer))
  (`/Game/Chess/BP_Pawn.ALL_setVals` bp_pawn slot moved enabled NewLocation GeometryCollection playerMove type))

(event `ALL_Restart`
  (bind _outactors (`GameplayStatics.GetAllActorsOfClass` "/Game/Chess/BP_ChessSlot.BP_ChessSlot_C"))
  (for _array_element _outactors
    (`/Game/Chess/BP_ChessSlot.setDefaults` _array_element))
  (`WidgetLayoutLibrary.RemoveAllWidgets`)
  (bind _outactors_2 (`GameplayStatics.GetAllActorsOfClass` "/Game/Chess/BP_Pawn.BP_Pawn_C"))
  (for _array_element_2 _outactors_2
    (`/Game/Chess/BP_Pawn.setDefaults` _array_element_2))
  (bind _aspc_chess (cast `/Game/Chess/PC_Chess` (`GameplayStatics.GetPlayerController` 0)))
  (set `/Game/Chess/PC_Chess.started` true _aspc_chess)
  (bind _returnvalue (`GameplayStatics.SpawnSound2D` "/Game/SFX/Ingame_BGM.Ingame_BGM" 1.0 1.0 0.0 null))
  (set `/Game/Chess/PC_Chess.BGM` _returnvalue _aspc_chess))

(event `setValuesSlot`
  (params (`Bp chess slot` :type "/Game/Chess/BP_ChessSlot Object Reference") (piecePawn :type "/Game/Chess/BP_Pawn Object Reference") (piece :type Boolean) (isWhite :type Boolean) (passant :type Boolean))
  (`/Game/Chess/BP_ChessSlot.setValues` `Bp chess slot` piecePawn piece isWhite passant))

(fn `updatePlayers`
  (params (playerMove :type Boolean) (pawn :type "/Game/Chess/BP_Pawn Object Reference"))
  (bind _outactors (`GameplayStatics.GetAllActorsOfClass` "/Game/Chess/BP_Pawn.BP_Pawn_C"))
  (for _array_element _outactors
    (bind _result (`/Engine/EditorBlueprintResources/StandardMacros.IncrementInt` (`/Game/Chess/BP_Pawn.lastReplicated` _array_element))
      (:`  `
        (if (or (== (mod _result 4) 0) (< (`/Game/Chess/BP_Pawn.moveTime` _array_element) 1.5))
          (bind (_slot _moved _enabled _returnvalue _geometrycollection _type) (`/Game/Chess/BP_Pawn.getValues` _array_element))
          (`self.setValuesThing` _array_element _slot _moved _enabled _returnvalue _geometrycollection false _type)))))
  (return))

(fn `updateSlots`
  (bind _outactors (`GameplayStatics.GetAllActorsOfClass` "/Game/Chess/BP_ChessSlot.BP_ChessSlot_C"))
  (for _array_element _outactors
    (bind _result (`/Engine/EditorBlueprintResources/StandardMacros.IncrementInt` (`/Game/Chess/BP_ChessSlot.modulo` _array_element))
      (:`  `
        (if (or (== (mod _result 4) 0) (< (`/Game/Chess/BP_ChessSlot.changeTimer` _array_element) 1.5))
          (bind (_piece _piecepawn _iswhite _passant) (`/Game/Chess/BP_ChessSlot.getValues` _array_element))
          (`self.setValuesSlot` _array_element _piecepawn _piece _iswhite _passant)))))
  (return))

(fn `UserConstructionScript`)