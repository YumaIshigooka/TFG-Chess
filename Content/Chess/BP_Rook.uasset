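; Rook chess piece Blueprint that handles hover, selection and moving between board slots, with movement rules still stubbed out.
; Cursor hover toggles custom-depth rendering, while Select swaps the material and highlights ValidSlots.
; Move updates slot occupancy, snaps the actor to the slot, clears highlights and calls UpdateValidSlots.
; UpdateValidSlots has an empty loop, CheckValidity always returns false, and an interpolated movement path is left unconnected.
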(event `self.ReceiveBeginPlay`
  (bind _aspc_chess (cast `/Game/Chess/PC_Chess` (`GameplayStatics.GetPlayerController` 0)))
  (set `self.playerController` _aspc_chess)
  (add `self.OnBeginCursorOver` (delegate `hoverStart`))
  (add `self.OnEndCursorOver` (delegate `hoverEnd`))
  (set `self.defaultMaterial` (`PrimitiveComponent.GetMaterial` (`self.Mesh`) 0))
  (`self.updateValidSlots`))

(event `hoverEnd` :!signature `self.OnEndCursorOver`
  (params (TouchedActor :type "Actor Object Reference"))
  (`PrimitiveComponent.SetRenderCustomDepth` (`self.Mesh`) false)
  (set `self.hovering` (not (`self.hovering`)))
  (set `/Game/Chess/PC_Chess.currPîeceHover` null (`self.playerController`)))

(event `hoverStart` :!signature `self.OnBeginCursorOver`
  (params (TouchedActor :type "Actor Object Reference"))
  (`PrimitiveComponent.SetRenderCustomDepth` (`self.Mesh`) true)
  (set `self.hovering` (not (`self.hovering`)))
  (set `/Game/Chess/PC_Chess.currPîeceHover` null (`self.playerController`)))

(event `self.move`
  (params (slot :type "/Game/Chess/BP_ChessSlot Object Reference"))
  (`/Game/Chess/BP_ChessSlot.setPieceOver` (`self.slot`) false false null)
  (bind _output_get (set `self.slot` slot))
  (`/Game/Chess/BP_ChessSlot.setPieceOver` _output_get false false null)
  (`self.K2_SetActorLocation` (+ (`self.K2_GetActorLocation` _output_get) (0.0 0.0 0.0)))
  (`self.highlightValidSlots` false)
  (`self.updateValidSlots`))

(event `self.highlightValidSlots`
  (params (highlight :type Boolean))
  (bind _result (`BlueprintSetLibrary.Set_ToArray` (`self.validSlots`)))
  (for _array_element _result
    (`/Game/Chess/BP_ChessSlot.highlight` _array_element highlight)))

(event `self.select`
  (bind _output_get (set `self.selected` (not (`self.selected`))))
  (if _output_get
    (`PrimitiveComponent.SetMaterial` (`self.Mesh`) 0 "/Engine/MapTemplates/Materials/BasicAsset03.BasicAsset03")
    (else
      (`PrimitiveComponent.SetMaterial` (`self.Mesh`) 0 (`self.defaultMaterial`))))
  (`self.highlightValidSlots` _output_get))

(event `self.updateValidSlots`
  (for _ (`/Game/Chess/PC_Chess.slots` (`self.playerController`))
    (if true
      _)))

(fn `checkValidity`
  (params (currSlot :type Integer) (newSlot :type Integer) (moved :type Boolean))
  (returns (ReturnValue :type Boolean))
  (return false))

(fn `UserConstructionScript`)