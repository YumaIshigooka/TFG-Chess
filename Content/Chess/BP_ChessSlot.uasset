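; BP_ChessSlot is one chess board square, tracking its occupying piece, colour and passant flag, with saved defaults for resetting.
; It sets a checker material on BeginPlay and swaps it to highlight.
; Hovering enables custom depth on squares valid for the controller's current piece and records the hovered slot.
; Placing a piece clears all highlights and captures any occupant via Geometry Collection physics, playing a gong for type 5, otherwise a capture sound plus cleanup.
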(event `initDefaults`
  (set `self.defaultPawn` (`self.piecePawn`))
  (set `self.defaultWhite` (`self.isWhite`))
  (set `self.defaultPiece` (`self.piece`)))

(event `setDefaults`
  (set `self.highlighted` false)
  (set `self.piecePawn` (`self.defaultPawn`))
  (set `self.isWhite` (`self.defaultWhite`))
  (set `self.piece` (`self.defaultPiece`)))

(event `self.ReceiveBeginPlay`
  (bind _plane (`self.Plane`))
  (`self.initDefaults`)
  (bind _aspc_chess (cast `/Game/Chess/PC_Chess` (`GameplayStatics.GetPlayerController` 0)))
  (set `self.PlayerController` _aspc_chess)
  (if (`self.isBlackSlot`)
    (`PrimitiveComponent.SetMaterial` _plane 0 "/Game/Chess/Materials/Textures/WhiteTile.WhiteTile")
    (else
      (`PrimitiveComponent.SetMaterial` _plane 0 "/Game/Chess/Materials/Textures/BlackTile.BlackTile")))
  (add `self.OnBeginCursorOver` (delegate `hoverStart`))
  (add `self.OnEndCursorOver` (delegate `hoverEnd`))
  (set `self.defaultMaterial` (`PrimitiveComponent.GetMaterial` (`self.Plane`) 0)))

(event `hoverStart` :!signature `self.OnBeginCursorOver`
  (params (TouchedActor :type "Actor Object Reference"))
  (bind _currpiece (`/Game/Chess/PC_Chess.currPiece` (`self.PlayerController`)))
  (`/Engine/EditorBlueprintResources/StandardMacros.IsValid` _currpiece
    (:`Is Valid`
      (if (`BlueprintSetLibrary.Set_Contains` (`/Game/Chess/BP_Pawn.validSlots` _currpiece) self)
        (`/Engine/EditorBlueprintResources/StandardMacros.IsValid` (`/Game/Chess/PC_Chess.currPiece` (`self.PlayerController`))
          (:`Is Valid`
            (`PrimitiveComponent.SetRenderCustomDepth` (`self.Plane`) true)
            (set `/Game/Chess/PC_Chess.currSlotHover` self (`self.PlayerController`))))))))

(event `hoverEnd` :!signature `self.OnEndCursorOver`
  (params (TouchedActor :type "Actor Object Reference"))
  (`PrimitiveComponent.SetRenderCustomDepth` (`self.Plane`) false)
  (set `/Game/Chess/PC_Chess.currSlotHover` null (`self.PlayerController`)))

(event `setValues`
  (params (piecePawn :type "/Game/Chess/BP_Pawn Object Reference") (piece :type Boolean) (isWhite :type Boolean) (passant :type Boolean))
  (set `self.piecePawn` piecePawn)
  (set `self.piece` piece)
  (set `self.isWhite` isWhite)
  (set `self.passant` passant))

(event `setBreakablePiece`
  (bind _piecepawn (`self.piecePawn`))
  (`PrimitiveComponent.SetSimulatePhysics` (`/Game/Chess/BP_Pawn.GeometryCollection` _piecepawn) true)
  (set `/Game/Chess/BP_Pawn.slot` null _piecepawn)
  (set `/Game/Chess/BP_Pawn.enabled` false _piecepawn)
  (`SceneComponent.K2_SetRelativeLocation` (`/Game/Chess/BP_Pawn.Widget` _piecepawn) (-100.0 -100.0 -450.0) false false)
  (clear `self.OnBeginCursorOver` _piecepawn)
  (if (!= (`/Game/Chess/BP_Pawn.type` _piecepawn) 5)
    (`GameplayStatics.PlaySound2D` "/Game/SFX/EatPiece.EatPiece" 1.0 1.0 0.0 null null)
    (`/Game/Chess/BP_Pawn.trashCollector` _piecepawn)
    (else
      (`GameplayStatics.PlaySound2D` "/Game/SFX/kungFu/gong.gong" 1.0 1.0 0.0 null null))))

(event `MULTI_setValues`
  (params (piecePawn :type "/Game/Chess/BP_Pawn Object Reference") (piece :type Boolean))
  (`self.setValues` piecePawn piece))

(event `highlight`
  (params (highlighted :type Boolean))
  (bind _output_get (set `self.highlighted` highlighted))
  (if _output_get
    (`PrimitiveComponent.SetMaterial` (`self.Plane`) 0 "/Engine/MapTemplates/Materials/BasicAsset03.BasicAsset03")
    (else
      (`PrimitiveComponent.SetMaterial` (`self.Plane`) 0 (`self.defaultMaterial`)))))

(event `deHighlightAllSlots`
  (bind _outactors (`GameplayStatics.GetAllActorsOfClass` "BP_ChessSlot_C"))
  (for _array_element _outactors
    (`self.highlight` _array_element false)))

(event `setPieceOver`
  (params (isWhite :type Boolean) (piece :type Boolean) (piecePawn :type "/Game/Chess/BP_Pawn Object Reference"))
  (set `self.piece` piece)
  (set `self.isWhite` isWhite)
  (`self.deHighlightAllSlots`)
  (if piece
    (`/Engine/EditorBlueprintResources/StandardMacros.IsValid` (`self.piecePawn`)
      (:`Is Valid`
        (`self.deHighlightAllSlots`)
        (`self.setBreakablePiece`))
      (:`Is Not Valid`
        _)))
  (bind _output_get (set `self.piecePawn` piecePawn))
  (`/Engine/EditorBlueprintResources/StandardMacros.IsValid` _output_get
    (:`Is Not Valid`
      (set `self.piece` false))))

(fn `getIndex`
  (params (row :type Integer) (col :type Integer))
  (returns (index :type Integer))
  (return (+ (* (- row 1) 8) (- col 1))))

(fn `getValues`
  (returns (piece :type Boolean) (piecePawn :type "/Game/Chess/BP_Pawn Object Reference") (isWhite :type Boolean) (passant :type Boolean))
  (return (`self.piece`) (`self.piecePawn`) (`self.isWhite`) (`self.passant`)))

(fn `isWhiteSlotFunc`
  (returns (ReturnValue :type Boolean))
  (return (not (`self.isBlackSlot`))))

(fn `UserConstructionScript`)