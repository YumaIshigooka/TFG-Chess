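; Chess bishop piece actor that toggles an outline on hover, swaps material when selected and highlights its candidate board slots.
; Move snaps it to a slot and recomputes valid moves by matching every BP_ChessSlot against a set of board indices computed from row and column.
; The per-index move test SubF is an empty stub, so bishop movement rules are absent; an interpolated movement path is left disconnected.
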(event `self.ReceiveBeginPlay`
  (bind _aspc_chess (cast `/Game/Chess/PC_Chess` (`GameplayStatics.GetPlayerController` 0)))
  (set `self.playerController` _aspc_chess)
  (add `self.OnBeginCursorOver` (delegate `hoverStart`))
  (add `self.OnEndCursorOver` (delegate `hoverEnd`))
  (set `self.defaultMaterial` (`PrimitiveComponent.GetMaterial` (`self.Mesh`) 0))
  (`self.updateValidSlots`))

(event `hoverEnd` :!signature `self.OnEndCursorOver`
  (params (TouchedActor :type "Actor Object Reference"))
  (`PrimitiveComponent.SetRenderCustomDepth` (`self.Mesh`) false)
  (set `self.hovering` (not (`self.hovering`)))
  (set `/Game/Chess/PC_Chess.currPîeceHover` null (`self.playerController`)))

(event `hoverStart` :!signature `self.OnBeginCursorOver`
  (params (TouchedActor :type "Actor Object Reference"))
  (`PrimitiveComponent.SetRenderCustomDepth` (`self.Mesh`) true)
  (set `self.hovering` (not (`self.hovering`)))
  (set `/Game/Chess/PC_Chess.currPîeceHover` null (`self.playerController`)))

(event `self.move`
  (params (slot :type "/Game/Chess/BP_ChessSlot Object Reference"))
  (`/Game/Chess/BP_ChessSlot.setPieceOver` (`self.slot`) false false null)
  (bind _output_get (set `self.slot` slot))
  (`/Game/Chess/BP_ChessSlot.setPieceOver` _output_get false false null)
  (`self.K2_SetActorLocation` (+ (`self.K2_GetActorLocation` _output_get) (0.0 0.0 0.0)))
  (`self.highlightValidSlots` false)
  (`self.updateValidSlots`))

(event `self.highlightValidSlots`
  (params (highlight :type Boolean))
  (bind _result (`BlueprintSetLibrary.Set_ToArray` (`self.validSlots`)))
  (for _array_element _result
    (`/Game/Chess/BP_ChessSlot.highlight` _array_element highlight)))

(event `self.select`
  (bind _output_get (set `self.selected` (not (`self.selected`))))
  (if _output_get
    (`PrimitiveComponent.SetMaterial` (`self.Mesh`) 0 "/Engine/MapTemplates/Materials/BasicAsset03.BasicAsset03")
    (else
      (`PrimitiveComponent.SetMaterial` (`self.Mesh`) 0 (`self.defaultMaterial`))))
  (`self.highlightValidSlots` _output_get))

(event `self.updateValidSlots`
  (bind _slot (`self.slot`))
  (`BlueprintSetLibrary.Set_Clear` (`self.validSlotId`))
  (`self.getValidSlotsID` (+ (* (- (`/Game/Chess/BP_ChessSlot.row` _slot) 1) 8) (`/Game/Chess/BP_ChessSlot.col` _slot)))
  (`BlueprintSetLibrary.Set_Clear` (`self.validSlots`))
  (bind _outactors (`GameplayStatics.GetAllActorsOfClass` "/Game/Chess/BP_ChessSlot.BP_ChessSlot_C"))
  (for _array_element _outactors
    (bind _returnvalue (`self.checkValidity` (`self.slot`) _array_element))
    (if _returnvalue
      (`BlueprintSetLibrary.Set_Add` (`self.validSlots`) _array_element)))
  (bind _result (`BlueprintSetLibrary.Set_ToArray` (`self.validSlotId`)))
  (for _array_element_2 _result
    (`KismetSystemLibrary.PrintString` (`KismetStringLibrary.Conv_IntToString` _array_element_2)))
  (`KismetSystemLibrary.PrintString` "Ended"))

(fn `checkValidity`
  (params (currSlot :type "/Game/Chess/BP_ChessSlot Object Reference") (newSlot :type "/Game/Chess/BP_ChessSlot Object Reference") (moved :type Boolean))
  (returns (ReturnValue :type Boolean))
  (return (`BlueprintSetLibrary.Set_Contains` (`self.validSlotId`) (+ (`/Game/Chess/BP_ChessSlot.col` newSlot) (* (- (`/Game/Chess/BP_ChessSlot.row` newSlot) 1) 8)))))

(fn `getValidSlotsID`
  (params (currSum :type Integer))
  (for _index (range 1 66)
    (bind _valid_ (`self.subF` (> currSum _index) currSum _index))
    (if _valid_
      (`BlueprintSetLibrary.Set_Add` (`self.validSlotId`) _index)))
  (`KismetSystemLibrary.PrintString` "Computado")
  (return))

(fn `subF`
  (params (greater :type Boolean) (currPos :type Integer) (newPos :type Integer))
  (returns (`valid?` :type Boolean))
  (locals (currPosTmp :type Integer) (newPosTmp7 :type Integer) (newPosTmp9 :type Integer)))

(fn `UserConstructionScript`)