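; BP_BoxThing is a box actor that the local player can hover and select while playing.
; On BeginPlay it caches the controlled BP_PawnThing and binds cursor events; hover enables custom depth on the cube and registers the box as the pawn's CurrBox.
; SERVER_selectThis forwards to selectThis, which marks it selected and swaps material, while clickThis deselects it.
; A BPP_Server lookup exists in initServer, but nothing here calls it.
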(event `initServer`
  (bind _outactors (`GameplayStatics.GetAllActorsOfClass` "/Game/BPP_Server.BPP_Server_C"))
  (set `self.Server` (`|GetArrayItem` _outactors)))

(event `self.ReceiveBeginPlay`
  (bind _returnvalue (`GameplayStatics.GetPlayerController` 0))
  (`/Engine/EditorBlueprintResources/StandardMacros.IsValid` _returnvalue
    (:`Is Valid`
      (bind _asbp_pawn_thing (cast `/Game/BP_PawnThing` (`Controller.K2_GetPawn` _returnvalue)))
      (set `self.myPlayer` _asbp_pawn_thing)
      (add `self.OnBeginCursorOver` (delegate `hoverStart`))
      (add `self.OnEndCursorOver` (delegate `hoverEnd`)))))

(event `hoverStart` :!signature `self.OnBeginCursorOver`
  (params (TouchedActor :type "Actor Object Reference"))
  (if (`/Game/BP_PawnThing.isPlaying` (`self.myPlayer`))
    (`PrimitiveComponent.SetRenderCustomDepth` (`self.Cube`) true)
    (set `self.isCursorOver` true)
    (set `/Game/BP_PawnThing.currBox` self (`self.myPlayer`))))

(event `hoverEnd` :!signature `self.OnEndCursorOver`
  (params (TouchedActor :type "Actor Object Reference"))
  (`PrimitiveComponent.SetRenderCustomDepth` (`self.Cube`) false)
  (set `self.isCursorOver` false))

(event `boxComm`
  (`KismetSystemLibrary.PrintString` "boxComm"))

(event `SERVER_selectThis`
  (`self.selectThis`))

(event `selectThis`
  (`KismetSystemLibrary.PrintString` "i got selected!" false)
  (set `self.isSelected` true)
  (`PrimitiveComponent.SetMaterial` (`self.Cube`) 0 "/Engine/MapTemplates/Materials/BasicAsset03.BasicAsset03"))

(event `clickThis`
  (set `self.isSelected` false)
  (`PrimitiveComponent.SetMaterial` (`self.Cube`) 0 "/Engine/MapTemplates/Materials/BasicAsset02.BasicAsset02"))

(fn `NewFunction`)

(fn `UserConstructionScript`)